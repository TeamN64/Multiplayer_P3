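; BP_NPC is a wandering NPC that uses AIMoveTo to head for random PuntoLLegada actors.
; BeginPlay gathers those exits and the Spawn actors, and Tick picks a new destination whenever velocity is zero.
; TocarSalida teleports the NPC to a random Spawn and sends it off again.
; Box overlap and hit events are empty, leaving the projectile ragdoll-and-destroy and NPC re-route logic disconnected.
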(event `self.ReceiveBeginPlay`
  (`self.Encontrar`)
  (bind _outactors (`GameplayStatics.GetAllActorsOfClass` "/Game/Carlos/PuntoLLegada.PuntoLLegada_C"))
  (for (_ _array_index) _outactors
    (set `self.num` _array_index))
  (bind _output (`|GetArrayItem` _outactors (`KismetMathLibrary.RandomIntegerInRange` 0 (`self.num`))))
  (`|AIMoveTo` self (`self.K2_GetActorLocation` _output) _output :!label _label))

(event `EncontrarSalida`
  (goto _label))

(event `self.ReceiveTick`
  (params (DeltaSeconds :type "Float (single-precision)"))
  (if (== (`self.GetVelocity`) (0.0 0.0 0.0))
    (`self.EncontrarSalida`)))

(event `self.Box.OnComponentBeginOverlap`
  (params (OverlappedComponent :type "PrimitiveComponent Object Reference") (OtherActor :type "Actor Object Reference") (OtherComp :type "PrimitiveComponent Object Reference") (OtherBodyIndex :type Integer) (bFromSweep :type Boolean) (SweepResult :type "HitResult Structure (by ref)")))

(event `Encontrar`
  (bind _outactors (`GameplayStatics.GetAllActorsOfClass` "/Game/Carlos/Spawn.Spawn_C"))
  (for (_ _array_index) _outactors
    (set `self.num2` _array_index)))

(event `TocarSalida`
  (`self.K2_SetActorLocation` (`self.K2_GetActorLocation` (`|GetArrayItem` (stale `Encontrar` _outactors) (`KismetMathLibrary.RandomIntegerInRange` 0 (`self.num2`)))) false true)
  (`self.EncontrarSalida`))

(event `self.Box.OnComponentHit`
  (params (HitComponent :type "PrimitiveComponent Object Reference") (OtherActor :type "Actor Object Reference") (OtherComp :type "PrimitiveComponent Object Reference") (NormalImpulse :type "Vector Structure") (Hit :type "HitResult Structure (by ref)"))
  ;[1 1 1] Conectar
)

(fn `UserConstructionScript`)