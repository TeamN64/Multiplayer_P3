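; Enemy AI character that shoots and chases the player, registering itself in the game mode's AmountAlive count.
; When PawnSensing spots the player, it turns to face them and, on a cooldown, calls AI MoveTo and fires.
; Each shot spawns a projectile with sound and muzzle effect, but also applies damage directly to the player.
; Depleted health triggers ragdoll, then delayed destruction and a decrement of AmountAlive.
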(event `self.ReceiveTick`
  (params (DeltaSeconds :type "Float (single-precision)"))
  (if (not (`self.isSeeingPlayer?`))
    (`MovementComponent.StopMovementImmediately` (`self.CharacterMovement`))))

(event `self.PawnSensing.OnSeePawn`
  (params (Pawn :type "Pawn Object Reference"))
  (bind _asbp_first_person_character (cast `/Game/FirstPerson/Blueprints/BP_FirstPersonCharacter` Pawn))
  (set `self.isSeeingPlayer?` true)
  (`GameplayStatics.PlaySoundAtLocation` "/Game/Felipe/EnemyAI/AISounds/AIDialog.AIDialog" (0.0 0.0 0.0) (struct) 1.0 1.0 0.0 null null null null)
  (`self.K2_SetActorRotation` (`KismetMathLibrary.FindRelativeLookAtRotation` (`KismetMathLibrary.Conv_VectorToTransform` (`self.K2_GetActorLocation`)) (`self.K2_GetActorLocation` _asbp_first_person_character)))
  (if (`self.canattack?`)
    (`self.FollowPlayer`)
    (if (not (<= (`self.HealthAI`) 0.0))
      (`|SpawnActorFromClass` "/Game/FirstPerson/Blueprints/BP_FirstPersonProjectileIA.BP_FirstPersonProjectileIA_C" (`SceneComponent.K2_GetComponentToWorld` (`self.SpawnP`)) "Undefined" "MultiplyWithRoot" null null)
      (`GameplayStatics.PlaySound2D` "/Game/Felipe/EnemyAI/AISounds/machine-gun-129929.machine-gun-129929" 1.0 1.0 0.0 null null)
      (`GameplayStatics.SpawnEmitterAttached` "/Game/FXVarietyPack/Particles/P_ky_shotShockwave.P_ky_shotShockwave" (`self.Flash`) "None" (0.0 0.0 0.0) (struct :`Yaw` 90.0) (0.03 0.03 0.03))
      (`GameplayStatics.ApplyDamage` _asbp_first_person_character 4.0)
      (set `self.canattack?` false)
      (`KismetSystemLibrary.Delay` 1.0)
      (set `self.canattack?` true))))

(event `FollowPlayer`
  (if (`self.isSeeingPlayer?`)
    (`|AIMoveTo` self (0.0 0.0 0.0) (`GameplayStatics.GetPlayerCharacter` 0) 70.0)
    (else
      (set `self.isSeeingPlayer?` false))))

(event `self.ReceiveBeginPlay`
  (bind _asbp_first_person_game_mode (cast `/Game/FirstPerson/Blueprints/BP_FirstPersonGameMode` (`GameplayStatics.GetGameMode`)))
  (set `/Game/FirstPerson/Blueprints/BP_FirstPersonGameMode.AmountAlive` (+ (`/Game/FirstPerson/Blueprints/BP_FirstPersonGameMode.AmountAlive` _asbp_first_person_game_mode) 1) _asbp_first_person_game_mode))

(event `self.ReceiveAnyDamage`
  (params (Damage :type "Float (single-precision)") (DamageType :type "DamageType Object Reference") (InstigatedBy :type "Controller Object Reference") (DamageCauser :type "Actor Object Reference"))
  (set `self.HealthAI` (- (`self.HealthAI`) Damage))
  (if (<= (`self.HealthAI`) 0.0)
    (`MovementComponent.StopMovementImmediately` (`self.CharacterMovement`))
    (`PrimitiveComponent.SetSimulatePhysics` (`self.Mesh`) true)
    (`KismetSystemLibrary.Delay` 3.0)
    (`self.K2_DestroyActor`)
    (bind _asbp_first_person_game_mode (cast `/Game/FirstPerson/Blueprints/BP_FirstPersonGameMode` (`GameplayStatics.GetGameMode`)))
    (set `/Game/FirstPerson/Blueprints/BP_FirstPersonGameMode.AmountAlive` (- (`/Game/FirstPerson/Blueprints/BP_FirstPersonGameMode.AmountAlive` _asbp_first_person_game_mode) 1) _asbp_first_person_game_mode)
    (else
      (`KismetSystemLibrary.PrintString` (`KismetStringLibrary.Conv_DoubleToString` (`self.HealthAI`)) true true (struct :`R` 1.0 :`B` 1.0 :`A` 1.0)))))

(event `self.Box.OnComponentHit`
  (params (HitComponent :type "PrimitiveComponent Object Reference") (OtherActor :type "Actor Object Reference") (OtherComp :type "PrimitiveComponent Object Reference") (NormalImpulse :type "Vector Structure") (Hit :type "HitResult Structure (by ref)")))

(fn `UserConstructionScript`)